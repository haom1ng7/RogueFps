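; BP_Battle1 is a roguelike battle room that initializes with node and floor index 0 and activates on BeginPlay.
; Activation only waits briefly before marking the room completed; door locking and enemy spawning are noted in a comment but not implemented.
; On completion it notifies the RunStateSubsystem, then spawns a BP_Portal for each next-depth choice at ChoicePointA or B, passing the target node ID and type label.
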(event EventBeginPlay
  (Class|RoomBase|InitializeRoom)
  (Class|RoomBase|ActivateRoom))

(event EventOnRoomActivated
  ;[0.15 0.15 0.15 0.5] 关门、上锁、刷怪
  (Utilities|FlowControl|Delay 5.0)
  (Class|RoomBase|MarkCompleted))

(event EventOnRoomCompleted
  (Class|RunStateSubsystem|NotifyRoomCompleted (Subsystems|GetRunStateSubsystem))
  (for (_array_element _array_index) (Class|RunStateSubsystem|GetChoicesforCurrentDepth (Subsystems|GetRunStateSubsystem))
    (Game|SpawnActorfromClass "/Game/Blueprints/Rooms/BP_Portal.BP_Portal_C" (Utilities|Select :Index _array_index :Option%200 (Transformation|GetActorTransform (Variables|Default|GetChoicePointA)) :Option%201 (Transformation|GetActorTransform (Variables|Default|GetChoicePointB))) "Undefined" "MultiplyWithRoot" 0 (.Id (Utilities|Struct|BreakRoomNode _array_element)) (|GenerictoText (.Type (Utilities|Struct|BreakRoomNode _array_element))) 0)))

(fn ConstructionScript)